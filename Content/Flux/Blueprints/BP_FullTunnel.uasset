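; BP_FullTunnel is a tunnel actor that travels along X and jumps ahead when the Flux character enters its trigger, apparently to recycle it as scrolling scenery.
; Tick moves the root with sweep at Movespeed scaled by world delta seconds.
; When BP_FluxCharacter overlaps the Box, the root teleports a large fixed distance in positive X and a debug string prints.
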(event `self.ReceiveTick`
  (params (DeltaSeconds :type "Float (single-precision)"))
  (bind _defaultsceneroot (`self.DefaultSceneRoot`))
  (bind (_relativelocation_x _relativelocation_y _relativelocation_z) (`KismetMathLibrary.BreakVector` (`SceneComponent.RelativeLocation` _defaultsceneroot)))
  (`SceneComponent.K2_SetRelativeLocation` _defaultsceneroot (`KismetMathLibrary.MakeVector` (+ _relativelocation_x (* (`self.movespeed`) (`GameplayStatics.GetWorldDeltaSeconds`))) _relativelocation_y _relativelocation_z) true false))

(event `self.Box.OnComponentBeginOverlap`
  (params (OverlappedComponent :type "PrimitiveComponent Object Reference") (OtherActor :type "Actor Object Reference") (OtherComp :type "PrimitiveComponent Object Reference") (OtherBodyIndex :type Integer) (bFromSweep :type Boolean) (SweepResult :type "HitResult Structure (by ref)"))
  (bind _defaultsceneroot (`self.DefaultSceneRoot`))
  (bind (_relativelocation_x _relativelocation_y _relativelocation_z) (`KismetMathLibrary.BreakVector` (`SceneComponent.RelativeLocation` _defaultsceneroot)))
  (cast `/Game/Flux/Blueprints/BP_FluxCharacter` OtherActor)
  (`SceneComponent.K2_SetRelativeLocation` _defaultsceneroot (`KismetMathLibrary.MakeVector` (+ _relativelocation_x 300000.0) _relativelocation_y _relativelocation_z) false true)
  (`KismetSystemLibrary.PrintString` "TUNNELLLL"))

(fn `UserConstructionScript`)