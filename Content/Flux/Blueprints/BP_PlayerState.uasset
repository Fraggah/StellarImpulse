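; Player state that tracks the player's total score and a capped Flow meter.
; BeginPlay caches the BP_PlayerController, and AddPoints raises TotalScore and fires the OnScoreChanged notification.
; AddFlow accumulates Flow up to MaxFlow and has the controller show the Space indicator when full.
; ConsumeFlow empties the meter and hides that indicator.
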(event `self.ReceiveBeginPlay`
  (bind _asbp_player_controller (cast `/Game/Flux/Blueprints/BP_PlayerController` (`self.GetPlayerController`)))
  (set `self.PlayerController` _asbp_player_controller))

(event `Add Points`
  (params (Points :type Integer))
  (set `self.TotalScore` (+ Points (`self.TotalScore`)))
  (`self.OnScoreChanged`))

(event `AddFlow`
  (params (Flow :type "Float (double-precision)"))
  (bind _maxflow (`self.MaxFlow`))
  (bind _returnvalue (+ (`self.Flow`) Flow))
  (bind _output_get (set `self.Flow` (`KismetMathLibrary.SelectFloat` _maxflow _returnvalue (> _returnvalue _maxflow))))
  (if (>= _output_get _maxflow)
    (`/Game/Flux/Blueprints/BP_PlayerController.ShowSpace` (`self.PlayerController`) true)))

(event `ConsumeFlow`
  (set `self.Flow` 0.0)
  (`/Game/Flux/Blueprints/BP_PlayerController.ShowSpace` (`self.PlayerController`) false))

(fn `UserConstructionScript`)