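; Player character for Flux that moves sideways between five lanes from the game mode's trail positions.
; Direct-lane and left/right step inputs drive timeline lerps with mesh roll-turns, locked while stepping; only left/right steps update the lane index.
; Damage drains PlayerState health with camera shake and material flash, pausing into Game Over at zero.
; Coin pickups pulse post-process; Nitro spends full Flow for brief slow motion.
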(event `EnhancedInput|/Game/Flux/Input/5T_IA`
  (params (ActionValue :type Boolean) (ElapsedSeconds :type "Float (double-precision)") (TriggeredSeconds :type "Float (double-precision)") (InputAction :type "InputAction Object Reference" :default "/Game/Flux/Input/5T_IA.5T_IA"))
  (bind (_returnvalue_x _returnvalue_y _returnvalue_z) (`KismetMathLibrary.BreakVector` (`self.K2_GetActorLocation`)))
  (bind _actualyposition (`self.ActualYPosition`))
  (bind _output (`|GetArrayItem` (`/Game/Flux/Blueprints/BP_FluxGameMode.TrailsPositionArray` (`self.Flux Game Mode`)) 4))
  ;[1 1 1] Movement System
  (:`Triggered`
    (if (`self.bIsSteping`)
      _
      (elif (not (== _output _actualyposition))
        (set `self.bIsSteping` true)
        (`self.RotateFlux` (> _actualyposition _output))
        (bind (_direction _alfa) (`Timeline|Timeline_2` :!via `PlayFromStart`)
          (:`Update`
            (`self.K2_SetActorLocation` (`KismetMathLibrary.MakeVector` _returnvalue_x (`KismetMathLibrary.Lerp` _actualyposition _output _alfa) _returnvalue_z)))
          (:`Finished`
            (set `self.ActualYPosition` _output)
            (set `self.bIsSteping` false)))))))

(event `EnhancedInput|/Game/Flux/Input/4R_IA`
  (params (ActionValue :type Boolean) (ElapsedSeconds :type "Float (double-precision)") (TriggeredSeconds :type "Float (double-precision)") (InputAction :type "InputAction Object Reference" :default "/Game/Flux/Input/4R_IA.4R_IA"))
  (bind (_returnvalue_x _returnvalue_y _returnvalue_z) (`KismetMathLibrary.BreakVector` (`self.K2_GetActorLocation`)))
  (bind _actualyposition (`self.ActualYPosition`))
  (bind _output (`|GetArrayItem` (`/Game/Flux/Blueprints/BP_FluxGameMode.TrailsPositionArray` (`self.Flux Game Mode`)) 3))
  ;[1 1 1] Movement System
  (:`Triggered`
    (if (`self.bIsSteping`)
      _
      (elif (not (== _output _actualyposition))
        (set `self.bIsSteping` true)
        (`self.RotateFlux` (> _actualyposition _output))
        (bind (_direction _alfa) (`Timeline|Timeline_1` :!via `PlayFromStart`)
          (:`Update`
            (`self.K2_SetActorLocation` (`KismetMathLibrary.MakeVector` _returnvalue_x (`KismetMathLibrary.Lerp` _actualyposition _output _alfa) _returnvalue_z)))
          (:`Finished`
            (set `self.ActualYPosition` _output)
            (set `self.bIsSteping` false)))))))

(event `EnhancedInput|/Game/Flux/Input/3E_IA`
  (params (ActionValue :type Boolean) (ElapsedSeconds :type "Float (double-precision)") (TriggeredSeconds :type "Float (double-precision)") (InputAction :type "InputAction Object Reference" :default "/Game/Flux/Input/3E_IA.3E_IA"))
  (bind (_returnvalue_x _returnvalue_y _returnvalue_z) (`KismetMathLibrary.BreakVector` (`self.K2_GetActorLocation`)))
  (bind _actualyposition (`self.ActualYPosition`))
  (bind _output (`|GetArrayItem` (`/Game/Flux/Blueprints/BP_FluxGameMode.TrailsPositionArray` (`self.Flux Game Mode`)) 2))
  ;[1 1 1] Movement System
  (:`Triggered`
    (if (`self.bIsSteping`)
      _
      (elif (not (== _output _actualyposition))
        (set `self.bIsSteping` true)
        (`self.RotateFlux` (> _actualyposition _output))
        (bind (_direction _alfa) (`Timeline|Timeline_0` :!via `PlayFromStart`)
          (:`Update`
            (`self.K2_SetActorLocation` (`KismetMathLibrary.MakeVector` _returnvalue_x (`KismetMathLibrary.Lerp` _actualyposition _output _alfa) _returnvalue_z)))
          (:`Finished`
            (set `self.ActualYPosition` _output)
            (set `self.bIsSteping` false)))))))

(event `EnhancedInput|/Game/Flux/Input/2W_IA`
  (params (ActionValue :type Boolean) (ElapsedSeconds :type "Float (double-precision)") (TriggeredSeconds :type "Float (double-precision)") (InputAction :type "InputAction Object Reference" :default "/Game/Flux/Input/2W_IA.2W_IA"))
  (bind (_returnvalue_x _returnvalue_y _returnvalue_z) (`KismetMathLibrary.BreakVector` (`self.K2_GetActorLocation`)))
  (bind _actualyposition (`self.ActualYPosition`))
  (bind _output (`|GetArrayItem` (`/Game/Flux/Blueprints/BP_FluxGameMode.TrailsPositionArray` (`self.Flux Game Mode`)) 1))
  ;[1 1 1] Movement System
  (:`Triggered`
    (if (`self.bIsSteping`)
      _
      (elif (not (== _output _actualyposition))
        (set `self.bIsSteping` true)
        (`self.RotateFlux` (> _actualyposition _output))
        (bind (_direction _alfa) (`Timeline|Timeline` :!via `PlayFromStart`)
          (:`Update`
            (`self.K2_SetActorLocation` (`KismetMathLibrary.MakeVector` _returnvalue_x (`KismetMathLibrary.Lerp` _actualyposition _output _alfa) _returnvalue_z)))
          (:`Finished`
            (set `self.ActualYPosition` _output)
            (set `self.bIsSteping` false)))))))

(event `self.ReceiveBeginPlay`
  (bind (_returnvalue_x _returnvalue_y _returnvalue_z) (`KismetMathLibrary.BreakVector` (`self.K2_GetActorLocation`)))
  (bind _mesh (`self.Mesh`))
  (bind _output (`|GetArrayItem` (`/Game/Flux/Blueprints/BP_FluxGameMode.TrailsPositionArray` (`self.Flux Game Mode`)) (`self.ActualIndexPosition`)))
  ;[1 1 1] Begin Play
  (bind _asbp_flux_game_mode (cast `/Game/Flux/Blueprints/BP_FluxGameMode` (`GameplayStatics.GetGameMode`)))
  (set `self.Flux Game Mode` _asbp_flux_game_mode)
  (bind _asbp_player_controller (cast `/Game/Flux/Blueprints/BP_PlayerController` (`self.GetController`)))
  (bind _returnvalue (pcsubsystem `EnhancedInputLocalPlayerSubsystem` _asbp_player_controller))
  (`/Engine/EditorBlueprintResources/StandardMacros.IsValid` _returnvalue
    (:`Is Valid`
      (`EnhancedInputSubsystemInterface.AddMappingContext` _returnvalue "/Game/Flux/Input/IMC_FluxDefault.IMC_FluxDefault" 0 (struct))
      (`self.K2_SetActorLocation` (`KismetMathLibrary.MakeVector` _returnvalue_x _output _returnvalue_z))
      (set `self.ActualYPosition` _output)
      (set `self.OriginalScale` (`SceneComponent.RelativeScale3D` (`self.Mesh`)))
      (bind _returnvalue_2 (`PrimitiveComponent.CreateDynamicMaterialInstance` _mesh 1 (`PrimitiveComponent.GetMaterial` _mesh 1) "None"))
      (set `self.FluxMaterial` _returnvalue_2)
      (bind _asbp_player_controller_2 (cast `/Game/Flux/Blueprints/BP_PlayerController` (`GameplayStatics.GetPlayerController` 0)))
      (set `self.Player Controller` _asbp_player_controller_2)
      (bind _asbp_player_state (cast `/Game/Flux/Blueprints/BP_PlayerState` (`GameplayStatics.GetPlayerState` 0)))
      (set `self.Player State` _asbp_player_state))))

(event `EnhancedInput|/Game/Flux/Input/1Q_IA`
  (params (ActionValue :type Boolean) (ElapsedSeconds :type "Float (double-precision)") (TriggeredSeconds :type "Float (double-precision)") (InputAction :type "InputAction Object Reference" :default "/Game/Flux/Input/1Q_IA.1Q_IA"))
  (bind (_returnvalue_x _returnvalue_y _returnvalue_z) (`KismetMathLibrary.BreakVector` (`self.K2_GetActorLocation`)))
  (bind _actualyposition (`self.ActualYPosition`))
  (bind _output (`|GetArrayItem` (`/Game/Flux/Blueprints/BP_FluxGameMode.TrailsPositionArray` (`self.Flux Game Mode`))))
  ;[1 1 1] Movement System
  (:`Triggered`
    (if (`self.bIsSteping`)
      _
      (elif (not (== _actualyposition _output))
        (set `self.bIsSteping` true)
        (`self.RotateFlux` true)
        (bind (_direction _alfa) (`Timeline|Step` :!via `PlayFromStart`)
          (:`Update`
            (`self.K2_SetActorLocation` (`KismetMathLibrary.MakeVector` _returnvalue_x (`KismetMathLibrary.Lerp` _actualyposition _output _alfa) _returnvalue_z)))
          (:`Finished`
            (set `self.ActualYPosition` _output)
            (set `self.bIsSteping` false)))))))

(event `EnhancedInput|/Game/Flux/Input/RightStep_IA`
  (params (ActionValue :type Boolean) (ElapsedSeconds :type "Float (double-precision)") (TriggeredSeconds :type "Float (double-precision)") (InputAction :type "InputAction Object Reference" :default "/Game/Flux/Input/RightStep_IA.RightStep_IA"))
  (bind (_returnvalue_x _returnvalue_y _returnvalue_z) (`KismetMathLibrary.BreakVector` (`self.K2_GetActorLocation`)))
  (bind _actualyposition (`self.ActualYPosition`))
  (bind _returnvalue (+ (`self.ActualIndexPosition`) 1))
  (bind _output (`|GetArrayItem` (`/Game/Flux/Blueprints/BP_FluxGameMode.TrailsPositionArray` (`self.Flux Game Mode`)) _returnvalue))
  (:`Triggered`
    (if (< _returnvalue 5)
      (if (`self.bIsSteping`)
        _
        (elif (not (== _actualyposition _output))
          (set `self.bIsSteping` true)
          (`self.RotateFlux` false)
          (bind (_direction _alfa) (`Timeline|Timeline_4` :!via `PlayFromStart`)
            (:`Update`
              (`self.K2_SetActorLocation` (`KismetMathLibrary.MakeVector` _returnvalue_x (`KismetMathLibrary.Lerp` _actualyposition _output _alfa) _returnvalue_z)))
            (:`Finished`
              (set `self.ActualYPosition` _output)
              (set `self.ActualIndexPosition` _returnvalue)
              (set `self.bIsSteping` false))))))))

(event `TakeDamageEffect`
  (bind _player_state (`self.Player State`))
  (bind _healthonhit (`self.HealthOnHit`))
  ;[1 1 1] Take Damage
  (`GameplayStatics.PlaySound2D` "/Game/Flux/Sounds/si_sound_hurt.si_sound_hurt" 1.0 1.0 0.0 null null)
  (set `self.HealthOnHit` (`/Game/Flux/Blueprints/BP_PlayerState.Health` (`self.Player State`)))
  (bind (_direction _newtrack_1) (`Timeline|Timeline_7` :!via `PlayFromStart`)
    (:`Update`
      (set `/Game/Flux/Blueprints/BP_PlayerState.Health` (`KismetMathLibrary.Lerp` _healthonhit (+ _healthonhit -7.0) _newtrack_1) _player_state)
      (if (<= (`/Game/Flux/Blueprints/BP_PlayerState.Health` _player_state) 0.0)
        (`self.Death Secuence`)))))

(event `RotateFlux`
  (params (`RotateTo Left` :type Boolean))
  (bind _rotationamount (`self.RotationAmount`))
  ;[1 1 1] Movement Rotation Anim
  (bind _output_get (set `self.StartRotation` (`SceneComponent.RelativeRotation` (`self.Mesh`))))
  (set `self.TargetRotation` (`KismetMathLibrary.MakeRotator` (.roll _output_get) (+ (.pitch _output_get) (`KismetMathLibrary.SelectFloat` (* _rotationamount -1.0) _rotationamount `RotateTo Left`)) (.yaw _output_get)))
  (bind (_direction _rot) (`Timeline|Timeline_3` :!via `PlayFromStart`)
    (:`Update`
      (`SceneComponent.K2_SetRelativeRotation` (`self.Mesh`) (`KismetMathLibrary.RLerp` (`self.StartRotation`) (`self.TargetRotation`) _rot true) false false))))

(event `Death Secuence`
  (bind _player_controller (`self.Player Controller`))
  ;[1 1 1] Death Secuence
  (`GameplayStatics.SetGamePaused` true)
  (bind _returnvalue (`|CreateWidget` "/Game/Flux/UI/Widget_GameOver.Widget_GameOver_C"))
  (`UserWidget.AddToViewport` _returnvalue 0)
  (`WidgetBlueprintLibrary.SetInputMode_UIOnlyEx` _player_controller null)
  (set `PlayerController.bShowMouseCursor` true _player_controller))

(event `EnhancedInput|/Game/Flux/Input/LeftStep_IA`
  (params (ActionValue :type Boolean) (ElapsedSeconds :type "Float (double-precision)") (TriggeredSeconds :type "Float (double-precision)") (InputAction :type "InputAction Object Reference" :default "/Game/Flux/Input/LeftStep_IA.LeftStep_IA"))
  (bind (_returnvalue_x _returnvalue_y _returnvalue_z) (`KismetMathLibrary.BreakVector` (`self.K2_GetActorLocation`)))
  (bind _actualyposition (`self.ActualYPosition`))
  (bind _returnvalue (+ (`self.ActualIndexPosition`) -1))
  (bind _output (`|GetArrayItem` (`/Game/Flux/Blueprints/BP_FluxGameMode.TrailsPositionArray` (`self.Flux Game Mode`)) _returnvalue))
  (:`Triggered`
    (if (>= _returnvalue 0)
      (if (`self.bIsSteping`)
        _
        (elif (not (== _actualyposition _output))
          (set `self.bIsSteping` true)
          (`self.RotateFlux` true)
          (bind (_direction _alfa) (`Timeline|Timeline_6` :!via `PlayFromStart`)
            (:`Update`
              (`self.K2_SetActorLocation` (`KismetMathLibrary.MakeVector` _returnvalue_x (`KismetMathLibrary.Lerp` _actualyposition _output _alfa) _returnvalue_z)))
            (:`Finished`
              (set `self.ActualYPosition` _output)
              (set `self.ActualIndexPosition` _returnvalue)
              (set `self.bIsSteping` false))))))))

(event `/Game/Flux/Blueprints/Interfaces/BPI_Block.TakeDamage`
  ;[1 1 1] Take Damage Effect
  (`self.TakeDamageEffect`)
  (`PlayerCameraManager.StartCameraShake` :`self` (`GameplayStatics.GetPlayerCameraManager` 0) :`ShakeClass` "/Game/Flux/Blueprints/BP_Camera_Shake.BP_Camera_Shake_C" :`Scale` 5.0 :`PlaySpace` "World")
  (`MaterialInstanceDynamic.SetVectorParameterValue` (`self.FluxMaterial`) "Color" (struct :`R` 0.225694 :`G` 0.020879 :`A` 1.0))
  (`KismetSystemLibrary.Delay` 0.5)
  (`MaterialInstanceDynamic.SetVectorParameterValue` (`self.FluxMaterial`) "Color" (struct :`G` 0.029557 :`B` 1.0 :`A` 1.0)))

(event `Coin Pickup Effect`
  ;[1 1 1] Coin Pickup Effect
  (bind (_direction _amount) (`Timeline|Timeline_5` :!via `PlayFromStart`)
    (:`Update`
      (set `PostProcessComponent.BlendWeight` _amount (`self.PostProcessCoin`)))))

(event `EnhancedInput|/Game/Flux/Input/NitroOn_IA`
  (params (ActionValue :type Boolean) (ElapsedSeconds :type "Float (double-precision)") (TriggeredSeconds :type "Float (double-precision)") (InputAction :type "InputAction Object Reference" :default "/Game/Flux/Input/NitroOn_IA.NitroOn_IA"))
  ;[1 1 1] Flux
  (:`Triggered`
    (if (and ActionValue (>= (`/Game/Flux/Blueprints/BP_PlayerState.Flow` (`self.Player State`)) 100.0))
      (`/Game/Flux/Blueprints/BP_PlayerState.ConsumeFlow` (`self.Player State`))
      (set `self.bIsOnPulse` true)
      (`GameplayStatics.SetGlobalTimeDilation` 0.4)
      (set `PostProcessComponent.BlendWeight` 1.0 (`self.PostProcessPulso`))
      (`KismetSystemLibrary.Delay` 1.0)
      (`GameplayStatics.SetGlobalTimeDilation` 1.0)
      (set `PostProcessComponent.BlendWeight` 0.0 (`self.PostProcessPulso`)))))

(event `/Game/Flux/Blueprints/Interfaces/BPI_Coin.Pickup`
  ;[1 1 1] Coin Pickup Effect
  (`self.Coin Pickup Effect`))

(fn `UserConstructionScript`)