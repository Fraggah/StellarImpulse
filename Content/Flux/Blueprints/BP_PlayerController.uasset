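; Player controller for Flux that sets up the HUD, input mapping and pause menu.
; On BeginPlay it creates the HUD widget and adds the default Enhanced Input mapping context.
; The pause action pauses the game, opens the pause widget and switches to UI-only input with the cursor shown.
; A ShowSpace event forwards a visibility flag to the HUD.
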(event `self.ReceiveBeginPlay`
  (bind _returnvalue (`|CreateWidget` "/Game/Flux/UI/Widget_HUD.Widget_HUD_C"))
  (bind _output_get (set `self.HUD` _returnvalue))
  (`UserWidget.AddToViewport` _output_get 0)
  (`EnhancedInputSubsystemInterface.AddMappingContext` (subsystem `EnhancedInputLocalPlayerSubsystem`) "/Game/Flux/Input/IMC_FluxDefault.IMC_FluxDefault" 0 (struct)))

(event `EnhancedInput|/Game/Flux/Input/Pause_IA`
  (params (ActionValue :type Boolean) (ElapsedSeconds :type "Float (double-precision)") (TriggeredSeconds :type "Float (double-precision)") (InputAction :type "InputAction Object Reference" :default "/Game/Flux/Input/Pause_IA.Pause_IA"))
  (:`Triggered`
    (`GameplayStatics.SetGamePaused` true)
    (bind _returnvalue (`|CreateWidget` "/Game/Flux/UI/Widget_Pause.Widget_Pause_C"))
    (`UserWidget.AddToViewport` _returnvalue 0)
    (set `self.bShowMouseCursor` true)
    (`WidgetBlueprintLibrary.SetInputMode_UIOnlyEx` self null)))

(event `ShowSpace`
  (params (Bool :type Boolean))
  (`/Game/Flux/UI/Widget_HUD.Set Space Visible` (`self.HUD`) Bool))

(fn `UserConstructionScript`)