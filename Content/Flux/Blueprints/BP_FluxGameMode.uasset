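; Game mode for an endless runner that moves coins, obstacles and recycled floor actors along X while playing, and hides character and HUD otherwise.
; A Delay in Tick throttles spawning far ahead: an obstacle and coin in random lanes, with every fifth spawn a wall whose single gap holds a coin.
; Items far behind the character are destroyed.
; AddScoreFlux forwards score and flux to PlayerState and animates the HUD.
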(event `self.ReceiveBeginPlay`
  (bind _asbp_flux_character (cast `/Game/Flux/Blueprints/BP_FluxCharacter` (`GameplayStatics.GetPlayerPawn` 0)))
  (set `self.Flux Character` _asbp_flux_character)
  (bind _asbp_player_state (cast `/Game/Flux/Blueprints/BP_PlayerState` (`GameplayStatics.GetPlayerState` 0)))
  (set `self.PlayerState` _asbp_player_state)
  (bind _asbp_player_controller (cast `/Game/Flux/Blueprints/BP_PlayerController` (`GameplayStatics.GetPlayerController` 0)))
  (set `self.PlayerControlle` _asbp_player_controller)
  (bind _returnvalue (`|CreateWidget` "/Game/Flux/UI/Widget_Black.Widget_Black_C"))
  (`UserWidget.AddToViewport` _returnvalue 0)
  (bind _outactors (`GameplayStatics.GetAllActorsOfClass` "/Game/Flux/Blueprints/BP_InfiniteFloor.BP_InfiniteFloor_C"))
  (set `self.FloorArray` _outactors))

(event `self.ReceiveTick`
  (params (DeltaSeconds :type "Float (single-precision)"))
  (bind _flux_character (`self.Flux Character`))
  (bind _flux_character_2 (`self.Flux Character`))
  (bind _hud (`/Game/Flux/Blueprints/BP_PlayerController.HUD` (`self.PlayerControlle`)))
  (if (`self.IsPlaying`)
    (`self.Move Coins`)
    (`self.Move Obstacles`)
    (`self.MoveFloor`)
    (`Widget.SetVisibility` _hud "Visible")
    (`SceneComponent.SetVisibility` (`Character.Mesh` _flux_character_2) true false)
    (`SceneComponent.SetVisibility` (`/Game/Flux/Blueprints/BP_FluxCharacter.Niagara1` _flux_character_2) true false)
    (set `self.PlayerX` (+ (.x (.location (`self.GetTransform` _flux_character_2))) 50000.0))
    (`self.DestroyObstacle`)
    (`self.DestroyCoins`)
    (`KismetSystemLibrary.Delay` 0.7)
    (`/Engine/EditorBlueprintResources/StandardMacros.IncrementInt` (`self.Count`)
      (:`  `
        (if (== (`self.Count`) 5)
          (`self.SpawnWall`)
          (set `self.Count` 0)
          (else
            (`self.SpawnObstacle`)))))
    (else
      (`SceneComponent.SetVisibility` (`Character.Mesh` _flux_character) false false)
      (`SceneComponent.SetVisibility` (`/Game/Flux/Blueprints/BP_FluxCharacter.Niagara1` _flux_character) false false)
      (`Widget.SetVisibility` _hud "Hidden"))))

(fn `Add Score & Flux`
  (params (ScoreToAdd :type Integer) (FluxToAdd :type "Float (double-precision)"))
  (bind _playerstate (`self.PlayerState`))
  (`/Game/Flux/Blueprints/BP_PlayerState.Add Points` _playerstate ScoreToAdd)
  (`/Game/Flux/Blueprints/BP_PlayerState.AddFlow` _playerstate FluxToAdd)
  (`/Game/Flux/Blueprints/BP_PlayerController.AnimateScoreHUD` (`self.PlayerControlle`)))

(fn `DestroyCoins`
  (bind _returnvalue (`GameplayStatics.GetActorOfClass` "/Game/Flux/Blueprints/BP_FluxCharacter.BP_FluxCharacter_C"))
  (for _array_element (`self.CoinsArray`)
    (if (> (- (.x (.location (`self.GetTransform` _returnvalue))) (.x (.location (`self.GetTransform` _array_element)))) 5000.0)
      (`self.K2_DestroyActor` _array_element)
      (`KismetArrayLibrary.Array_RemoveItem` (`self.CoinsArray`) _array_element))))

(fn `DestroyObstacle`
  (bind _returnvalue (`GameplayStatics.GetActorOfClass` "/Game/Flux/Blueprints/BP_FluxCharacter.BP_FluxCharacter_C"))
  (for _array_element (`self.ObstaclesArray`)
    (if (> (- (.x (.location (`self.GetTransform` _returnvalue))) (.x (.location (`self.GetTransform` _array_element)))) 5000.0)
      (`self.K2_DestroyActor` _array_element)
      (`KismetArrayLibrary.Array_RemoveItem` (`self.ObstaclesArray`) _array_element))))

(fn `Move Coins`
  (bind _coinsarray (`self.CoinsArray`))
  (if (not (`KismetArrayLibrary.Array_IsEmpty` _coinsarray))
    (for _array_element _coinsarray
      (bind _defaultsceneroot (`/Game/Flux/Blueprints/BP_Coin.DefaultSceneRoot` _array_element))
      (bind (_relativelocation_x _relativelocation_y _relativelocation_z) (`KismetMathLibrary.BreakVector` (`SceneComponent.RelativeLocation` _defaultsceneroot)))
      (`SceneComponent.K2_SetRelativeLocation` _defaultsceneroot (`KismetMathLibrary.MakeVector` (+ _relativelocation_x (* (`self.ComponentsSpeed`) (`GameplayStatics.GetWorldDeltaSeconds`))) _relativelocation_y _relativelocation_z) false false))))

(fn `Move Obstacles`
  (bind _obstaclesarray (`self.ObstaclesArray`))
  (if (not (`KismetArrayLibrary.Array_IsEmpty` _obstaclesarray))
    (for _array_element _obstaclesarray
      (bind _rootcomponent (`Actor.RootComponent` _array_element))
      (bind (_relativelocation_x _relativelocation_y _relativelocation_z) (`KismetMathLibrary.BreakVector` (`SceneComponent.RelativeLocation` _rootcomponent)))
      (`SceneComponent.K2_SetRelativeLocation` _rootcomponent (`KismetMathLibrary.MakeVector` (+ _relativelocation_x (* (`self.ComponentsSpeed`) (`GameplayStatics.GetWorldDeltaSeconds`))) _relativelocation_y _relativelocation_z) false false))))

(fn `MoveFloor`
  (locals (FullFloorDistance :type "Float (double-precision)" :default 60000.0))
  (bind _fullfloordistance (`local.FullFloorDistance`))
  (for _array_element (`self.FloorArray`)
    (bind (_returnvalue_x _returnvalue_y _returnvalue_z) (`KismetMathLibrary.BreakVector` (`self.K2_GetActorLocation` _array_element)))
    (bind _returnvalue (+ (* (`self.ComponentsSpeed`) (`GameplayStatics.GetWorldDeltaSeconds`)) _returnvalue_x))
    (`self.K2_SetActorLocation` _array_element (`KismetMathLibrary.MakeVector` _returnvalue _returnvalue_y _returnvalue_z) false false)
    (if (< _returnvalue (- (`self.PlayerX`) _fullfloordistance))
      (`self.K2_SetActorLocation` _array_element (`KismetMathLibrary.MakeVector` (+ _returnvalue_x _fullfloordistance) _returnvalue_y _returnvalue_z) false false))))

(fn `SpawnObstacle`
  (locals (`Obstacle Pos` :type "Float (double-precision)"))
  (bind _output_get (set `local.Obstacle Pos` (`KismetArrayLibrary.Array_Random` (`self.PositionSpawnerArray`))))
  (`KismetArrayLibrary.Array_RemoveItem` (`self.PositionSpawnerArray`) _output_get)
  (bind _returnvalue (`|SpawnActorFromClass` "/Game/Flux/Blueprints/BP_Obstacle.BP_Obstacle_C" (`KismetMathLibrary.MakeTransform` (`KismetMathLibrary.MakeVector` (`self.PlayerX`) _output_get 1100.0)) "Undefined" "MultiplyWithRoot" null null))
  (`KismetArrayLibrary.Array_Add` (`self.ObstaclesArray`) _returnvalue)
  (bind _returnvalue_2 (`|SpawnActorFromClass` "/Game/Flux/Blueprints/BP_Coin.BP_Coin_C" (`KismetMathLibrary.MakeTransform` (`KismetMathLibrary.MakeVector` (`self.PlayerX`) (`KismetArrayLibrary.Array_Random` (`self.PositionSpawnerArray`)) (.z (.location (`self.GetTransform` (`self.Flux Character`)))))) "Undefined" "MultiplyWithRoot" null null))
  (`KismetArrayLibrary.Array_Add` (`self.CoinsArray`) _returnvalue_2)
  (`KismetArrayLibrary.Array_Add` (`self.PositionSpawnerArray`) (`local.Obstacle Pos`)))

(fn `SpawnWall`
  (bind _playerx (`self.PlayerX`))
  (bind _returnvalue (+ (`KismetArrayLibrary.Array_Length` (`self.PositionSpawnerArray`)) -1))
  (set `self.RandomIndex` (`KismetMathLibrary.RandomIntegerInRange` 0 _returnvalue))
  (for _index (range (+ _returnvalue 1))
    (if (== _index (`self.RandomIndex`))
      (bind _output (`|GetArrayItem` (`self.PositionSpawnerArray`) _index))
      (bind _returnvalue_2 (`|SpawnActorFromClass` "/Game/Flux/Blueprints/BP_Coin.BP_Coin_C" (`KismetMathLibrary.MakeTransform` (`KismetMathLibrary.MakeVector` _playerx _output (.z (.location (`self.GetTransform` (`self.Flux Character`)))))) "Undefined" "MultiplyWithRoot" null null))
      (`KismetArrayLibrary.Array_Add` (`self.CoinsArray`) _returnvalue_2)
      (else
        (bind _returnvalue_3 (`|SpawnActorFromClass` "/Game/Flux/Blueprints/BP_Obstacle.BP_Obstacle_C" (`KismetMathLibrary.MakeTransform` (`KismetMathLibrary.MakeVector` _playerx _output 1100.0)) "Undefined" "MultiplyWithRoot" null null))
        (`KismetArrayLibrary.Array_Add` (`self.ObstaclesArray`) _returnvalue_3)))))

(fn `UserConstructionScript`)